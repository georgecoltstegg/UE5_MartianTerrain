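; Interior prop Blueprint for a stack of nine cabinets in the Mars 2030 HDU, with configurable labels.
; The construction script assigns each of the nine label mesh components its own static mesh variable and applies a matching material variable to material slot 1.
; It has no runtime logic, as the event graph holds only disabled placeholder events.
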(fn `UserConstructionScript`
  (bind _sm_label_4 (`self.SM_Label_4`))
  (bind _sm_label_3 (`self.SM_Label_3`))
  (bind _sm_label_2 (`self.SM_Label_2`))
  (bind _sm_label_1 (`self.SM_Label_1`))
  (bind _sm_label_5 (`self.SM_Label_5`))
  (bind _sm_label_6 (`self.SM_Label_6`))
  (bind _sm_label_7 (`self.SM_Label_7`))
  (bind _sm_label_8 (`self.SM_Label_8`))
  (bind _sm_label_9 (`self.SM_Label_9`))
  (`StaticMeshComponent.SetStaticMesh` _sm_label_1 (`self.Label_1`))
  (`StaticMeshComponent.SetStaticMesh` _sm_label_2 (`self.Label_2`))
  (`StaticMeshComponent.SetStaticMesh` _sm_label_3 (`self.Label_3`))
  (`StaticMeshComponent.SetStaticMesh` _sm_label_4 (`self.Label_4`))
  (`StaticMeshComponent.SetStaticMesh` _sm_label_5 (`self.Label_5`))
  (`StaticMeshComponent.SetStaticMesh` _sm_label_6 (`self.Label_6`))
  (`StaticMeshComponent.SetStaticMesh` _sm_label_7 (`self.Label_7`))
  (`StaticMeshComponent.SetStaticMesh` _sm_label_8 (`self.Label_8`))
  (`StaticMeshComponent.SetStaticMesh` _sm_label_9 (`self.Label_9`))
  (`PrimitiveComponent.SetMaterial` _sm_label_1 1 (`self.Label_1_Mat`))
  (`PrimitiveComponent.SetMaterial` _sm_label_2 1 (`self.Label_2_Mat`))
  (`PrimitiveComponent.SetMaterial` _sm_label_3 1 (`self.Label_3_Mat`))
  (`PrimitiveComponent.SetMaterial` _sm_label_4 1 (`self.Label_4_Mat`))
  (`PrimitiveComponent.SetMaterial` _sm_label_5 1 (`self.Label_5_Mat`))
  (`PrimitiveComponent.SetMaterial` _sm_label_6 1 (`self.Label_6_Mat`))
  (`PrimitiveComponent.SetMaterial` _sm_label_7 1 (`self.Label_7_Mat`))
  (`PrimitiveComponent.SetMaterial` _sm_label_8 1 (`self.Label_8_Mat`))
  (`PrimitiveComponent.SetMaterial` _sm_label_9 1 (`self.Label_9_Mat`)))